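; BP_FieldSystem is a Chaos field actor that breaks apart and blasts geometry collections around its location when its Explode event is called.
; Explode first applies external cluster strain through a radial falloff sphere with no falloff to fracture clusters.
; It then applies a linear force from a radial vector, culled outside that same sphere and passed with a metadata filter, to push pieces outward from the actor.
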(event `Explode`
  (bind _returnvalue (`self.K2_GetActorLocation`))
  (bind _fieldsystemcomponent (`self.FieldSystemComponent`))
  (bind _returnvalue_2 (`RadialFalloff.SetRadialFalloff` (`self.RadialFalloff`) 1000000.0 0.0 1.0 0.0 200.0 _returnvalue "Field_FallOff_None"))
  (`FieldSystemComponent.ApplyPhysicsField` _fieldsystemcomponent true "Field_ExternalClusterStrain" null _returnvalue_2)
  (`FieldSystemComponent.ApplyPhysicsField` _fieldsystemcomponent true "Field_LinearForce" (`self.FieldSystemMetaDataFilter`) (`CullingField.SetCullingField` (`self.CullingField`) _returnvalue_2 (`RadialVector.SetRadialVector` (`self.RadialVector`) 7000000.0 _returnvalue) "Field_Culling_Outside")))

(event `self.ReceiveBeginPlay`)

(fn `UserConstructionScript`)