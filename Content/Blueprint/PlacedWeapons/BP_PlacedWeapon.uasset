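; BP_PlacedWeapon is a placed-weapon actor that generates Chaos physics fields to fracture and scatter destructible objects.
; CreateFields applies an external cluster strain through a radial falloff centered on the supplied location.
; It then applies an outward radial linear force, culled outside that sphere and using the field's filter metadata.
; The file holds no trigger logic, as BeginPlay, overlap and construction are empty.
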(event `self.ReceiveBeginPlay`)

(event `self.CreateFields`
  (params (FieldLocation :type "Vector Structure (by ref)"))
  (bind _returnvalue (`RadialFalloff.SetRadialFalloff` (`self.RadialFalloff`) 5000000.0 0.9 1.0 0.0 200.0 FieldLocation "Field_FallOff_None"))
  (`FieldSystemComponent.ApplyPhysicsField` (`self.FieldSystem`) true "Field_ExternalClusterStrain" null _returnvalue)
  (`FieldSystemComponent.ApplyPhysicsField` (`self.FieldSystem`) true "Field_LinearForce" (`self.FieldSystemMetaDataFilter`) (`CullingField.SetCullingField` (`self.CullingField`) _returnvalue (`RadialVector.SetRadialVector` (`self.RadialVector`) 1000000.0 FieldLocation) "Field_Culling_Outside")))

(fn `UserConstructionScript`)