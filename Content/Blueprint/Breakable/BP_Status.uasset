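; BP_Status is a breakable actor in the Breakable folder, extending a parent class that supplies the GetHit event and uses a Geometry Collection component.
; On GetHit it runs the parent's hit handling, then sets the Geometry Collection to ignore the Pawn channel so pawns are no longer blocked by it.
; It adds no other active logic, as its BeginPlay, overlap and Tick events are disabled placeholders.
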(event `self.GetHit`
  (params (ImpactPoint :type "Vector Structure (by ref)"))
  (`parent.GetHit` ImpactPoint)
  (`PrimitiveComponent.SetCollisionResponseToChannel` (`self.GeometryCollectionComponent`) "ECC_Pawn" "ECR_Ignore"))

(fn `UserConstructionScript`
  (`parent.UserConstructionScript`))